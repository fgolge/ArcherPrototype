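; BP_BaseCharacter is a character Blueprint that provides movement, look and jump controls plus data-driven class setup.
; Its construction script looks up Type in DT_BaseClasses to set max health, weapon type and max damage on the health and weapon components, printing an error if no row matches.
; Movement follows control rotation: forward uses yaw only, while right uses yaw and roll.
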(event Input|ActionEvents|InputActionJump
  (params (Key :type Key%20Structure))
  ;[1 1 1] InputAxis and Jump
  (:Pressed
    (Character|Jump))
  (:Released
    (Character|StopJumping)))

(event Input|AxisEvents|InputAxisMoveForward
  (params (AxisValue :type Float%20%28single-precision%29))
  ;[1 1 1] InputAxis and Jump
  (CallFunction|MoveForward AxisValue))

(event Input|AxisEvents|InputAxisLookUp
  (params (AxisValue :type Float%20%28single-precision%29))
  ;[1 1 1] InputAxis and Jump
  (Pawn|Input|AddControllerPitchInput AxisValue))

(event Input|AxisEvents|InputAxisLookRight
  (params (AxisValue :type Float%20%28single-precision%29))
  ;[1 1 1] InputAxis and Jump
  (Pawn|Input|AddControllerYawInput AxisValue))

(event Input|AxisEvents|InputAxisMoveRight
  (params (AxisValue :type Float%20%28single-precision%29))
  ;[1 1 1] InputAxis and Jump
  (CallFunction|MoveRight AxisValue))

(fn ConstructionScript
  (bind _ac_weaponcomponent (Variables|Default|GetAC_WeaponComponent))
  (bind _returnvalue (Utilities|GetDataTableRow "/Game/Data/CharacterData/DT_BaseClasses.DT_BaseClasses" (Variables|Default|GetType))
    (:then
      (Default|SetMaxHealth (Variables|Default|GetAC_HealthComponent) (.Health (Utilities|Struct|BreakF_BaseClassProperties _returnvalue)))
      (Default|UpdateWeaponType _ac_weaponcomponent (.WeaponType (Utilities|Struct|BreakF_BaseClassProperties _returnvalue)))
      (Default|SetMaxDamage _ac_weaponcomponent (.Damage (Utilities|Struct|BreakF_BaseClassProperties _returnvalue))))
    (:RowNotFound
      (Development|PrintString "Type wasn't found!" true true "(R=0.000000,G=0.660000,B=1.000000,A=1.000000)" 3e+01))))

(fn MoveForward
  (params (ScaleValue :type Float%20%28double-precision%29))
  (Pawn|Input|AddMovementInput (Math|Vector|GetForwardVector (Math|Rotator|MakeRotator 0.0 0.0 (.yaw (Pawn|GetControlRotation :!class /Script/Engine.Pawn)))) ScaleValue false))

(fn MoveRight
  (params (ScaleValue :type Float%20%28double-precision%29))
  (bind _returnvalue (Pawn|GetControlRotation :!class /Script/Engine.Pawn))
  (Pawn|Input|AddMovementInput (Math|Vector|GetRightVector (Math|Rotator|MakeRotator (.roll _returnvalue) 0.0 (.yaw _returnvalue))) ScaleValue false))